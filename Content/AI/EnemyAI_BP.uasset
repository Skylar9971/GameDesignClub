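; Base enemy AI character that senses targets and casts spells through SpellSystemBPC, with startup casts or levitation for certain elemental subclasses.
; PawnSensing and a NearSense overlap write the seen player or enemy to the Blackboard.
; Tick clamps velocity and rolls non-attack abilities via CheckAbilityCast, using range, random chance and a one-time low-health trigger.
; BeginPlay refreshes spell data from Spells_DT; AIMoveToLevitate steers flight and reports attack range.
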(event `self.ReceiveTick`
  (params (DeltaSeconds :type "Float (single-precision)"))
  (bind _charactermovement (`self.CharacterMovement`))
  (bind _maxvelocity (`self.MaxVelocity`))
  (set `MovementComponent.Velocity` (`KismetMathLibrary.ClampVectorSize` (`MovementComponent.Velocity` _charactermovement) (* _maxvelocity -1.0) _maxvelocity) _charactermovement)
  (bind (_relicindex _doability) (`self.CheckAbilityCast` false))
  (if _doability
    (`/Game/Spells/SpellSystem/SpellSystem_BPC.BeginCast` :`self` (`self.SpellSystem_BPC`) :`RelicIndex` _relicindex :`SpecificIndex` true :`InstaCast` true)))

(event `self.ReceiveBeginPlay`
  (bind _modifiers (`/Game/Spells/SpellSystem/SpellSystem_BPC.Modifiers` (`self.SpellSystem_BPC`)))
  (for (_ _array_index) _modifiers
    (bind _spellscasting (break `/Game/Spells/SpellSystem/ModifierInfo_S` (`|GetArrayItem` _modifiers _array_index)))
    (for (_array_element _array_index_2) _spellscasting
      (bind _returnvalue (`|GetDataTableRow` "/Game/Spells/SpellSystem/Spells_DT.Spells_DT" (`KismetStringLibrary.Conv_StringToName` (`|GetEnumeratorNameAsString` (`.SpellName_9_6C6976B44D6BD2719DA1B0B92918511B` (break `/Game/Spells/SpellSystem/SpellInfo_S` _array_element)))))
        (:`then`
          (`KismetArrayLibrary.Array_Set` _spellscasting _array_index_2 _returnvalue)))))
  (if (or (`GameplayStatics.ObjectIsA` self "/Game/AI/HeatwaveEnemy/HeatwaveEnemy_BP.HeatwaveEnemy_BP_C") (`GameplayStatics.ObjectIsA` self "/Game/AI/WaterEnemy/WaterEnemy_BP.WaterEnemy_BP_C"))
    (`/Game/Spells/SpellSystem/SpellSystem_BPC.BeginCast` :`self` (`self.SpellSystem_BPC`) :`RelicIndex` 1 :`SpecificIndex` true :`InstaCast` true))
  (if (`GameplayStatics.ObjectIsA` self "/Game/AI/WindEnemy/WindEnemy_BP.WindEnemy_BP_C")
    (`/Game/Spells/SpellSystem/SpellSystem_BPC.Levitate` (`self.SpellSystem_BPC`))))

(event `self.NearSense.OnComponentBeginOverlap`
  (params (OverlappedComponent :type "PrimitiveComponent Object Reference") (OtherActor :type "Actor Object Reference") (OtherComp :type "PrimitiveComponent Object Reference") (OtherBodyIndex :type Integer) (bFromSweep :type Boolean) (SweepResult :type "HitResult Structure (by ref)"))
  (bind _returnvalue (`AIBlueprintHelperLibrary.GetBlackboard` (`AIBlueprintHelperLibrary.GetAIController` self)))
  (bind _asbp_first_person_character (cast `/Game/FirstPerson/Blueprints/BP_FirstPersonCharacter` OtherActor)
    (:`then`
      (`BlackboardComponent.SetValueAsObject` _returnvalue "SeenPawn" _asbp_first_person_character)
      (`BlackboardComponent.SetValueAsBool` _returnvalue "HasSeenPlayer" true :!label _label))
    (:`CastFailed`
      (bind _asenemy_ai_bp (cast `/Game/AI/EnemyAI_BP` OtherActor))
      (if (!= _asenemy_ai_bp self)
        (`BlackboardComponent.SetValueAsObject` _returnvalue "SeenPawn" _asenemy_ai_bp)
        (goto _label)))))

(event `self.PawnSensing.OnSeePawn`
  (params (Pawn :type "Pawn Object Reference"))
  (bind _returnvalue (`AIBlueprintHelperLibrary.GetBlackboard` (`AIBlueprintHelperLibrary.GetAIController` self)))
  (`BlackboardComponent.SetValueAsBool` _returnvalue "HasSeenPlayer" true)
  (`BlackboardComponent.SetValueAsObject` _returnvalue "SeenPawn" Pawn))

(fn `AIMoveToLevitate`
  (params (TargetPawn :type "Pawn Object Reference") (TargetLocation :type "Vector Structure"))
  (returns (InRange :type Boolean))
  (bind _mtlcurlocation (`self.MTLCurLocation`))
  (bind _rootcomponent (`self.RootComponent`))
  (bind _returnvalue (`SceneComponent.K2_GetComponentLocation` _rootcomponent))
  (bind _returnvalue_2 (`KismetMathLibrary.FindLookAtRotation` _returnvalue _mtlcurlocation))
  (`/Engine/EditorBlueprintResources/StandardMacros.IsValid` TargetPawn
    (:`Is Valid`
      (set `self.MTLCurLocation` (`SceneComponent.K2_GetComponentLocation` (`Actor.RootComponent` TargetPawn))))
    (:`Is Not Valid`
      (set `self.MTLCurLocation` (`KismetMathLibrary.MakeVector` (.x TargetLocation) (.y TargetLocation) (.z _returnvalue)))))
  (set `MovementComponent.Velocity` (`KismetMathLibrary.MakeVector` (.x (* (`KismetMathLibrary.GetForwardVector` _returnvalue_2) (`self.LevitateSpeed`))) (.y (* (`KismetMathLibrary.GetForwardVector` _returnvalue_2) (`self.LevitateSpeed`))) (.z (* (`KismetMathLibrary.GetForwardVector` _returnvalue_2) (`self.LevitateSpeed`)))) (`self.CharacterMovement`))
  (`SceneComponent.K2_SetWorldRotation` _rootcomponent (`KismetMathLibrary.MakeRotator` 0.0 0.0 (.yaw _returnvalue_2)) false false)
  (return (<= (`KismetMathLibrary.Vector_Distance` _returnvalue _mtlcurlocation) (`self.AttackRadius`))))

(fn `CheckAbilityCast`
  (params (AttackAbility :type Boolean))
  (returns (RelicIndex :type Integer) (DoAbility :type Boolean))
  (bind _health (`self.Health`))
  (bind _returnvalue (`AIBlueprintHelperLibrary.GetBlackboard` (`AIBlueprintHelperLibrary.GetAIController` self)))
  (set `self.DoAbility` false)
  (set `self.AbilityCurIndex` 0)
  (for (_array_element _array_index) (`self.Abilities`)
    (bind (_abilityrange _noabilityrange _isattackability _lowhpability _abilitychance) (break `/Game/Spells/SpellSystem/Ability_S` _array_element))
    (if _noabilityrange
      (if (or (and _isattackability AttackAbility) (not _isattackability)) :!label _label
        (if (and (< (`/Game/FirstPerson/Blueprints/Health.Health` _health) (* (`/Game/FirstPerson/Blueprints/Health.MaxHealth` _health) _lowhpability)) (not (`self.LowHPCasted`)))
          (set `self.LowHPCasted` true)
          (set `self.AbilityCurIndex` (+ _array_index 1) :!label _label_2)
          (set `self.DoAbility` true)
          (elif (`KismetMathLibrary.RandomBoolWithWeight` _abilitychance)
            (goto _label_2))))
      (elif (`BlackboardComponent.GetValueAsBool` _returnvalue "HasSeenPlayer")
        (bind _aspawn (cast `Pawn` (`BlackboardComponent.GetValueAsObject` _returnvalue "SeenPawn")))
        (if (< (`self.GetDistanceTo` _aspawn self) _abilityrange)
          (goto _label)))))
  (return (`self.AbilityCurIndex`) (`self.DoAbility`)))

(fn `UserConstructionScript`)